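; Player controller that sets up the health bar HUD and handles pausing.
; On BeginPlay it creates the health bar widget and adds it to the viewport.
; The Pause input toggles game pause, showing or removing the pause menu and switching cursor visibility and input mode to match.
; The pause menu widget is created lazily on first use and cached for reuse.
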(event `self.ReceiveBeginPlay`
  ;[1 1 1] Здоровье
  (bind _returnvalue (`|CreateWidget` "/Game/UI/WBP_Healthbar.WBP_Healthbar_C" (`GameplayStatics.GetPlayerController` 0)))
  (`UserWidget.AddToViewport` _returnvalue 0))

(event `InputAction|Pause`
  (params (Key :type "Key Structure"))
  (:`Pressed`
    (if (`GameplayStatics.IsGamePaused`)
      (`WidgetBlueprintLibrary.SetInputMode_GameOnly` (`self.PlayerControllerRef`))
      (`Widget.RemoveFromParent` (`self.PauseMenuRef`))
      (`GameplayStatics.SetGamePaused` false)
      (set `PlayerController.bShowMouseCursor` false (`self.PlayerControllerRef`))
      (else
        (set `self.PlayerControllerRef` (`GameplayStatics.GetPlayerController` 0))
        (`/Engine/EditorBlueprintResources/StandardMacros.IsValid` (`self.PauseMenuRef`)
          (:`Is Valid`
            _)
          (:`Is Not Valid`
            (bind _returnvalue (`|CreateWidget` "/Game/UI/WBP_PauseMenu.WBP_PauseMenu_C"))
            (set `self.PauseMenuRef` _returnvalue)))
        (`WidgetBlueprintLibrary.SetInputMode_GameAndUIEx` (`self.PlayerControllerRef`) null)
        (set `PlayerController.bShowMouseCursor` true (`self.PlayerControllerRef`))
        (`UserWidget.AddToViewport` (`self.PauseMenuRef`) 0)
        (`GameplayStatics.SetGamePaused` true)))))

(fn `UserConstructionScript`)