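; BP_MeleeWeapon is a sword that deals melee damage and can be picked up by the main character.
; On BeginPlay it copies Damage from a parent BP_Enemy, while its sphere overlap hands it to BP_MainCharacter to attach, with a sound.
; Hitbox overlaps send damage through BP_WeaponInterface to actors of a different class than the wielder, gated by a short cooldown.
; The construction script configures mesh and hitbox; older direct-damage logic is unused.
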(event `self.ReceiveBeginPlay`
  (bind _asbp_enemy (cast `/Game/Blueprints/Enemy/BP_Enemy` (`self.GetAttachParentActor`)))
  (set `self.Damage` (`/Game/Blueprints/Enemy/BP_Enemy.Damage` _asbp_enemy)))

(event `self.ReceiveTick`
  (params (DeltaSeconds :type "Float (single-precision)")))

(event `self.HitBoxCollision.OnComponentBeginOverlap`
  (params (OverlappedComponent :type "PrimitiveComponent Object Reference") (OtherActor :type "Actor Object Reference") (OtherComp :type "PrimitiveComponent Object Reference") (OtherBodyIndex :type Integer) (bFromSweep :type Boolean) (SweepResult :type "HitResult Structure (by ref)"))
  (bind _returnvalue (`self.GetAttachParentActor`))
  (if (and (`KismetSystemLibrary.DoesImplementInterface` OtherActor "/Game/Blueprints/BP_WeaponInterface.BP_WeaponInterface_C") (!= (`GameplayStatics.GetObjectClass` OtherActor) (`GameplayStatics.GetObjectClass` _returnvalue)) (`self.CanDoDamage`) (!= _returnvalue null))
    (set `self.CanDoDamage` false)
    (message `/Game/Blueprints/BP_WeaponInterface.GetDamage` OtherActor (`self.Damage`))
    (`KismetSystemLibrary.Delay` 0.6)
    (set `self.CanDoDamage` true)))

(event `self.Sphere.OnComponentBeginOverlap`
  (params (OverlappedComponent :type "PrimitiveComponent Object Reference") (OtherActor :type "Actor Object Reference") (OtherComp :type "PrimitiveComponent Object Reference") (OtherBodyIndex :type Integer) (bFromSweep :type Boolean) (SweepResult :type "HitResult Structure (by ref)"))
  (bind _asbp_main_character (cast `/Game/Blueprints/BP_MainCharacter` OtherActor))
  (set `self.As BP Main Character` _asbp_main_character)
  (set `/Game/Blueprints/BP_MainCharacter.WeaponRef` self _asbp_main_character)
  (`/Game/Blueprints/BP_MainCharacter.AttachWeapon` _asbp_main_character)
  (`GameplayStatics.PlaySound2D` "/Game/FMOD/Assets/New_Folder/WeaponFX/weapon_ring.weapon_ring" 1.0 1.0 0.0 null null))

(fn `UserConstructionScript`
  (bind _staticmesh (`self.StaticMesh`))
  (bind _hitboxcollision (`self.HitBoxCollision`))
  (switch `int` (`self.NumberOfWeapon`)
    (:`Default`
      _)
    (:`0`
      _))
  (`BoxComponent.SetBoxExtent` _hitboxcollision (4.0 2.0 50.0) true)
  (`SceneComponent.K2_SetRelativeLocation` _hitboxcollision (0.0 0.0 -70.0) false true)
  (`StaticMeshComponent.SetStaticMesh` _staticmesh "/Game/Weapon_Pack/Mesh/Weapons/Weapons_Kit/SM_Sword.SM_Sword")
  (set `self.NameOfWeapon` "THSword")
  (`PrimitiveComponent.SetMaterial` _staticmesh 0 "/Game/Weapon_Pack/Materials/Weapons/M_WeaponSet_1.M_WeaponSet_1"))