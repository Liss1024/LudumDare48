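; Walking melee enemy that chases the player on AI perception and attacks up close.
; A looping timer keeps perception active at walk speed; the random-move node is unwired, and sighting clears the timer.
; AIMoveTo leads into AttackPlayer, which disables perception, slows movement, pulses IsAttacking and repeats while a debug-drawn sphere overlap finds the player.
; BeginPlay attaches the player controller's MeleeWeaponRef to its WeaponSocket; the final DoesSeePlayer1 result goes unused.
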(event `MoveToRandomLocation`
  (`ActorComponent.Activate` (`self.AIPerception`) false)
  (set `CharacterMovementComponent.MaxWalkSpeed` 200.0 (`self.CharacterMovement`)))

(event `StartWalking`)

(event `self.ReceiveBeginPlay`
  (bind _returnvalue (`KismetSystemLibrary.K2_SetTimerDelegate` (delegate `MoveToRandomLocation`) 2.0 true))
  (`KismetSystemLibrary.Delay` 0.2)
  (bind _asbp_main_player_controller (cast `/Game/Blueprints/BP_mainPlayerController` (`GameplayStatics.GetPlayerController` 0)))
  (bind _meleeweaponref (`/Game/Blueprints/BP_mainPlayerController.MeleeWeaponRef` _asbp_main_player_controller))
  (set `self.Melee Weapon Ref` _meleeweaponref)
  (`self.K2_AttachToComponent` _meleeweaponref (`self.Mesh`) "WeaponSocket" "SnapToTarget" "SnapToTarget" "KeepRelative" true))

(event `self.AIPerception.OnTargetPerceptionUpdated`
  (params (Actor :type "Actor Object Reference") (Stimulus :type "AIStimulus Structure"))
  ;[1 1 1] Если АИ заметит игрока, то побежит к нему
  (bind _asbp_main_character (cast `/Game/Blueprints/BP_MainCharacter` Actor))
  (set `self.As BP Main Character` _asbp_main_character)
  (`KismetSystemLibrary.K2_ClearAndInvalidateTimerHandle` (stale `self.ReceiveBeginPlay` _returnvalue) :!label _label)
  (set `CharacterMovementComponent.MaxWalkSpeed` 600.0 (`self.CharacterMovement`))
  (`AITask_MoveTo.AIMoveTo` (`AIBlueprintHelperLibrary.GetAIController` self) (0.0 0.0 0.0) _asbp_main_character 100.0 "Disable"
    (:`OnMoveFinished`
      (`self.ShouldAttackPlayer?`)
      (`self.AttackPlayer`))))

(event `RunToPlayer`
  ;[1 1 1] Если АИ заметит игрока, то побежит к нему
  (goto _label))

(event `AttackPlayer`
  (`ActorComponent.Deactivate` (`self.AIPerception`))
  (set `CharacterMovementComponent.MaxWalkSpeed` 50.0 (`self.CharacterMovement`))
  (set `self.IsAttacking` true)
  (`KismetSystemLibrary.RetriggerableDelay` 1.0)
  (set `self.IsAttacking` false)
  (bind _shouldattack (`self.ShouldAttackPlayer?`))
  (if _shouldattack
    (`self.AttackPlayer`)
    (`self.FailReport` "attack")
    (else
      (`self.DoesSeePlayer1`))))

(event `Death`
  (`self.K2_DestroyActor`))

(fn `DoesSeePlayer1`
  (returns (DoesSee :type Boolean))
  (bind _as_bp_main_character (`self.As BP Main Character`))
  (`/Engine/EditorBlueprintResources/StandardMacros.IsValid` _as_bp_main_character
    (:`Is Valid`
      (`/Engine/EditorBlueprintResources/StandardMacros.CompareInt` (`KismetArrayLibrary.Array_Find` (`AIPerceptionComponent.GetCurrentlyPerceivedActors` (`self.AIPerception`) null) _as_bp_main_character)
        (:`>`
          (return true))
        (:`==`
          (return true))
        (:`<`
          _)))
    (:`Is Not Valid`
      _))
  (return false))

(fn `ShouldAttackPlayer?`
  (returns (ShouldAttack :type Boolean))
  (bind _returnvalue (`self.K2_GetActorLocation`))
  (bind _melee_weapon_ref (`self.Melee Weapon Ref`))
  (`KismetSystemLibrary.DrawDebugSphere` _returnvalue 150.0 12 (struct :`R` 0.174959 :`G` 1.0 :`A` 1.0) 1.0 2.0)
  (`/Engine/EditorBlueprintResources/StandardMacros.IsValid` _melee_weapon_ref
    (:`Is Valid`
      (bind _outactors (`KismetSystemLibrary.SphereOverlapActors` _returnvalue 150.0 (`|MakeArray` "ObjectTypeQuery3" :!type "EObjectTypeQuery Enum") null (`|MakeArray` self _melee_weapon_ref :!type "Actor Object Reference")))
      (`/Engine/EditorBlueprintResources/StandardMacros.CompareInt` (`KismetArrayLibrary.Array_Find` _outactors (`self.As BP Main Character`))
        (:`>`
          _)
        (:`==`
          _)
        (:`<`
          (return false))))
    (:`Is Not Valid`
      (bind _outactors_2 (`KismetSystemLibrary.SphereOverlapActors` _returnvalue 150.0 (`|MakeArray` "ObjectTypeQuery3" :!type "EObjectTypeQuery Enum") null (`|MakeArray` self :!type "Actor Object Reference")))
      (`/Engine/EditorBlueprintResources/StandardMacros.CompareInt` (`KismetArrayLibrary.Array_Find` _outactors_2 (`self.As BP Main Character`))
        (:`>`
          _)
        (:`==`
          _)
        (:`<`
          (return false)))))
  (return true))

(fn `UserConstructionScript`)