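; Melee walking enemy that patrols, chases the player on sight, attacks or retreats, driven by Blueprint events and timers.
; It spawns a weapon into its hand socket and patrols random reachable points until AIPerception spots the player, then notifies the enemy manager.
; After moves or attacks, MakeDecision calls the manager's GiveOrders, then picks attack (if permitted and in range), retreat, chase or patrol.
; Attacks trigger through an AnimBP flag, with a timer polling for completion.
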(event `ShouldWalk`
  ;[1 1 1] Если АИ потерял игрока, то этот ивент отправит его патрулировать дальше
  (if (not (`KismetSystemLibrary.K2_IsTimerActiveHandle` (stale `StartWalking` _returnvalue)))
    (bind _doessee (`self.DoesSeePlayer`))
    (if (not _doessee)
      (`KismetSystemLibrary.RetriggerableDelay` 3.0)
      (bind _doessee_2 (`self.DoesSeePlayer`))
      (if (not _doessee_2)
        (`self.StartWalking`)))))

(event `MoveToRandomLocation`
  ;[1 1 1] Включаем AIPerception и идем в патруль
  (set `self.CanDetectPlayer` true)
  (set `CharacterMovementComponent.MaxWalkSpeed` 200.0 (`self.CharacterMovement`))
  (bind _doessee (`self.DoesSeePlayer`))
  (if (not _doessee)
    (`AIBlueprintHelperLibrary.SimpleMoveToLocation` (`AIBlueprintHelperLibrary.GetAIController` self) (`NavigationSystemV1.K2_GetRandomReachablePointInRadius` (`self.K2_GetActorLocation`) 1000.0 null null))))

(event `StartWalking`
  (bind _returnvalue (`KismetSystemLibrary.K2_SetTimerDelegate` (delegate `MoveToRandomLocation`) 2.0 true :!label _label)) ; Таймер для патрулирования. Отправляет в рандомную точку каждые 2 секунды
)

(event `self.ReceiveBeginPlay`
  (bind _returnvalue (`self.GetTransform`))
  (`|ExecutionSequence`
    (:`then_0`
      (`KismetSystemLibrary.K2_SetTimerDelegate` (delegate `ShouldWalk`) 4.0 true) ; Таймер для проверки, не стоит ли АИ как дурак без дела
      (goto _label))
    (:`then_1`
      ;[1 1 1] Спавним оружие и кидаем его в руку
      (bind _returnvalue_2 (`|SpawnActorFromClass` "/Game/Blueprints/BP_MeleeWeapon.BP_MeleeWeapon_C" (`KismetMathLibrary.MakeTransform` (`KismetMathLibrary.MakeVector` (.x (.location _returnvalue)) (.y (.location _returnvalue)) (- (.z (.location _returnvalue)) 200.0))) "AlwaysSpawn" "OverrideRootScale" null 0 null))
      (`self.K2_AttachToComponent` _returnvalue_2 (`self.Mesh`) "RightHandWeaponSocket" "SnapToTarget" "SnapToTarget" "SnapToTarget" true))
    (:`then_2`
      (`KismetSystemLibrary.Delay` 1.0)
      (bind _asbp_main_character (cast `/Game/Blueprints/BP_MainCharacter` (`GameplayStatics.GetPlayerCharacter` 0)))
      (bind _output_get (set `self.As BP Main Character` _asbp_main_character))
      (set `self.EnemyManagerRef` (`/Game/Blueprints/BP_MainCharacter.EnemyManagerRef` _output_get)))
    (:`then_3`
      (bind _asbp_game_instance (cast `/Game/Blueprints/Misc/BP_GameInstance` (`GameplayStatics.GetGameInstance`)))
      (set `/Game/Blueprints/Misc/BP_GameInstance.WalkingEnemyRef` self _asbp_game_instance))))

(event `self.AIPerception.OnTargetPerceptionUpdated`
  (params (Actor :type "Actor Object Reference") (Stimulus :type "AIStimulus Structure"))
  (bind _enemymanagerref (`self.EnemyManagerRef`))
  ;[1 1 1] Если АИ заметит игрока, то сообщит менеджеру
  (bind _asbp_main_character (cast `/Game/Blueprints/BP_MainCharacter` Actor))
  (set `self.As BP Main Character` _asbp_main_character)
  (if (`self.CanDetectPlayer`)
    (`/Engine/EditorBlueprintResources/StandardMacros.IsValid` _enemymanagerref
      (:`Is Valid`
        (`/Game/Blueprints/Enemy/BP_EnemyManager.OnEnemyTriggered` _enemymanagerref self)
        ;[1 1 1] Бежим к игроку
        (`KismetSystemLibrary.K2_ClearAndInvalidateTimerHandle` (stale `StartWalking` _returnvalue) :!label _label_2)
        (set `CharacterMovementComponent.MaxWalkSpeed` 600.0 (`self.CharacterMovement`))
        (`AITask_MoveTo.AIMoveTo` (`AIBlueprintHelperLibrary.GetAIController` self) (0.0 0.0 0.0) (`self.As BP Main Character`) 100.0 "Disable"
          (:`OnMoveFinished`
            (`self.MakeDecision`))))
      (:`Is Not Valid`
        (`self.FailReport` "Not Valid")))))

(event `RunToPlayer`
  ;[1 1 1] Бежим к игроку
  (goto _label_2))

(event `CheckIsAttackOver`
  (if (not (`self.IsAttacking`))
    (`KismetSystemLibrary.K2_ClearAndInvalidateTimerHandle` (stale `AttackPlayer` _returnvalue))
    (`KismetSystemLibrary.Delay` 0.2)
    (`self.MakeDecision`)))

(event `AttackPlayer`
  ;[1 1 1] Атакуем игрока
  (set `self.CanDetectPlayer` false)
  (set `CharacterMovementComponent.MaxWalkSpeed` 50.0 (`self.CharacterMovement`))
  (set `self.IsAttacking` true)
  (bind _aswalking_enemy_anim_bp (cast `/Game/Mannequin/Animations/WalkingEnemyAnimBP` (`SkeletalMeshComponent.GetAnimInstance` (`self.Mesh`))))
  (set `/Game/Mannequin/Animations/WalkingEnemyAnimBP.DoesSimpleAttack` true _aswalking_enemy_anim_bp)
  (bind _returnvalue (`KismetSystemLibrary.K2_SetTimerDelegate` (delegate `CheckIsAttackOver`) 0.2 true)))

(event `Death`
  ;[1 1 1] Смерть
  (for _array_element (`self.GetAttachedActors` true)
    (`self.K2_DestroyActor` _array_element))
  (`self.K2_DestroyActor`))

(event `Retreat`
  ;[1 1 1] Отступаем
  (set `self.CanDetectPlayer` false)
  (set `CharacterMovementComponent.MaxWalkSpeed` 100.0 (`self.CharacterMovement`))
  (`AITask_MoveTo.AIMoveTo` (`AIBlueprintHelperLibrary.GetAIController` self) (+ (* (- (`self.K2_GetActorLocation`) (`self.K2_GetActorLocation` (`self.As BP Main Character`))) 2) (`self.K2_GetActorLocation`)) null
    (:`OnRequestFailed`
      _)
    (:`OnMoveFinished`
      _))
  (set `self.CanDetectPlayer` true))

(event `MakeDecision`
  ;[1 1 1] Проверка что делать атаковать, отступать, бежать к игроку, патрулировать
  (`/Game/Blueprints/Enemy/BP_EnemyManager.GiveOrders` (`self.EnemyManagerRef`))
  (bind _shouldattack (`self.ShouldAttackPlayer?`))
  (if _shouldattack
    (`self.AttackPlayer`)
    (else
      (bind _doessee (`self.DoesSeePlayer`))
      (if _doessee
        (bind _shouldretreat (`self.ShouldRetreat`))
        (if _shouldretreat
          (`self.Retreat`)
          (else
            (`self.RunToPlayer`)))
        (else
          (`self.StartWalking`))))))

(event `self.ReceiveTick`
  (params (DeltaSeconds :type "Float (single-precision)"))
  (`KismetSystemLibrary.PrintString` (`KismetStringLibrary.Conv_BoolToString` (`self.IsAttacking`)) true true (struct :`G` 0.66 :`B` 1.0 :`A` 1.0) 0.0))

(fn `DoesSeePlayer`
  (returns (DoesSee :type Boolean))
  (bind _as_bp_main_character (`self.As BP Main Character`))
  (`/Engine/EditorBlueprintResources/StandardMacros.IsValid` _as_bp_main_character
    (:`Is Valid`
      (`/Engine/EditorBlueprintResources/StandardMacros.CompareInt` (`KismetArrayLibrary.Array_Find` (`AIPerceptionComponent.GetCurrentlyPerceivedActors` (`self.AIPerception`) null) _as_bp_main_character)
        (:`>`
          (return true))
        (:`==`
          (return true))
        (:`<`
          _)))
    (:`Is Not Valid`
      _))
  (return false))

(fn `ShouldAttackPlayer?`
  (returns (ShouldAttack :type Boolean))
  (bind _returnvalue (`self.K2_GetActorLocation`))
  (bind _melee_weapon_ref (`self.Melee Weapon Ref`))
  (if (`self.HasPermissionToAttack`)
    (`KismetSystemLibrary.DrawDebugSphere` _returnvalue 150.0 12 (struct :`R` 0.174959 :`G` 1.0 :`A` 1.0) 1.0 2.0)
    (`/Engine/EditorBlueprintResources/StandardMacros.IsValid` _melee_weapon_ref
      (:`Is Valid`
        (bind _outactors (`KismetSystemLibrary.SphereOverlapActors` _returnvalue 150.0 (`|MakeArray` "ObjectTypeQuery3" :!type "EObjectTypeQuery Enum") null (`|MakeArray` self _melee_weapon_ref :!type "Actor Object Reference")))
        (`/Engine/EditorBlueprintResources/StandardMacros.CompareInt` (`KismetArrayLibrary.Array_Find` _outactors (`self.As BP Main Character`))
          (:`>`
            _)
          (:`==`
            _)
          (:`<`
            (return false))))
      (:`Is Not Valid`
        (bind _outactors_2 (`KismetSystemLibrary.SphereOverlapActors` _returnvalue 150.0 (`|MakeArray` "ObjectTypeQuery3" :!type "EObjectTypeQuery Enum") null (`|MakeArray` self :!type "Actor Object Reference")))
        (`/Engine/EditorBlueprintResources/StandardMacros.CompareInt` (`KismetArrayLibrary.Array_Find` _outactors_2 (`self.As BP Main Character`))
          (:`>`
            _)
          (:`==`
            _)
          (:`<`
            (return false)))))
    (return true)
    (else
      (return false))))

(fn `ShouldRetreat`
  (returns (ShouldRetreat :type Boolean))
  (bind _as_bp_main_character (`self.As BP Main Character`))
  (`/Engine/EditorBlueprintResources/StandardMacros.IsValid` _as_bp_main_character
    (:`Is Valid`
      (return (>= 62500.0 (`KismetMathLibrary.VSizeXYSquared` (- (`self.K2_GetActorLocation` _as_bp_main_character) (`self.K2_GetActorLocation`))))))
    (:`Is Not Valid`
      (return false))))

(fn `UserConstructionScript`)