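; BP_EnemyManager tracks active and triggered enemies and controls which may attack the player.
; GiveOrders compacts null entries in the triggered list, sorts it, copies leading entries into AttackingEnemies and sets their HasPermissionToAttack, clearing it for later entries.
; The sort is an early-exit bubble sort comparing squared XY distance to the player, though its swaps write to ListOfActiveEnemies rather than the triggered list it compares.
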(event `self.ReceiveBeginPlay`
  (bind _asbp_main_character (cast `/Game/Blueprints/BP_MainCharacter` (`GameplayStatics.GetPlayerCharacter` 0)))
  (set `self.As BP Main Character` _asbp_main_character))

(event `AddEnemyToList`
  (params (NewEnemy :type "/Game/Blueprints/Enemy/BP_WalkingEnemy Object Reference"))
  (bind _currentnumberofenemies (`self.CurrentNumberOfEnemies`))
  (`KismetArrayLibrary.Array_Set` (`self.ListOfActiveEnemies`) _currentnumberofenemies NewEnemy true)
  (`/Engine/EditorBlueprintResources/StandardMacros.IncrementInt` _currentnumberofenemies))

(event `OnEnemyTriggered`
  (params (EnemyRef :type "/Game/Blueprints/Enemy/BP_WalkingEnemy Object Reference"))
  (bind _listoftriggeredenemies (`self.ListOfTriggeredEnemies`))
  (bind _numberoftriggeredenemies (`self.NumberOfTriggeredEnemies`))
  (`/Engine/EditorBlueprintResources/StandardMacros.CompareInt` (`KismetArrayLibrary.Array_Find` _listoftriggeredenemies EnemyRef)
    (:`<`
      (`KismetArrayLibrary.Array_Set` _listoftriggeredenemies _numberoftriggeredenemies EnemyRef true)
      (`/Engine/EditorBlueprintResources/StandardMacros.IncrementInt` _numberoftriggeredenemies))))

(event `GiveOrders`
  (bind _listoftriggeredenemies (`self.ListOfTriggeredEnemies`))
  (bind _attackingenemies (`self.AttackingEnemies`))
  ;[1 1 1] Очищаем массив от невалидных элементов, сортируем и записываем первые элементы в массив атакующих
  (`self.GetRidOfNULLInArray`)
  (`self.SortTriggeredEnemies` _listoftriggeredenemies)
  (for (_ _array_index) _attackingenemies
    (`KismetArrayLibrary.Array_Set` _attackingenemies _array_index (`|GetArrayItem` _listoftriggeredenemies _array_index))
    (for _array_element _attackingenemies
      (set `/Game/Blueprints/Enemy/BP_WalkingEnemy.HasPermissionToAttack` true _array_element)
      (for _index (range (- (`KismetArrayLibrary.Array_Length` (`self.AttackingEnemies`)) 1) (`KismetArrayLibrary.Array_Length` (`self.ListOfTriggeredEnemies`)))
        (set `/Game/Blueprints/Enemy/BP_WalkingEnemy.HasPermissionToAttack` false (`|GetArrayItem` (`self.ListOfTriggeredEnemies`) _index))))))

(fn `GetRidOfNULLInArray`
  (locals (N :type Integer :default 0))
  (bind _listoftriggeredenemies (`self.ListOfTriggeredEnemies`))
  (bind _listoftriggeredenemies_2 (`self.ListOfTriggeredEnemies`))
  ;[1 1 1] Проверяем каждый элемент массива, не равен ли он NULL
  (set `local.N` (- (`KismetArrayLibrary.Array_Length` _listoftriggeredenemies) 1))
  (for (_array_element _array_index) _listoftriggeredenemies
    (if (== _array_element null)
      ;[1 1 1] Если есть, то смещаем все после него на 1 к началу
      (for _index (range _array_index (+ (`local.N`) 1))
        (`KismetArrayLibrary.Array_Set` _listoftriggeredenemies_2 _index (`|GetArrayItem` _listoftriggeredenemies_2 (+ _index 1)) true))))
  ;[1 1 1] Обновляем количество активных врагов
  (set `self.NumberOfTriggeredEnemies` (- (`KismetArrayLibrary.Array_Length` (`self.ListOfTriggeredEnemies`)) 1)))

(fn `SortTriggeredEnemies`
  (params (ListOfTriggeredEnemies :type "Array of /Game/Blueprints/Enemy/BP_WalkingEnemy Object Reference"))
  (locals (N :type Integer) (SwapEnemy :type "/Game/Blueprints/Enemy/BP_WalkingEnemy Object Reference") (F :type Boolean))
  (bind _listofactiveenemies (`self.ListOfActiveEnemies`))
  (bind _output_get (set `local.N` (`KismetArrayLibrary.Array_Length` (`local.ListOfTriggeredEnemies`))))
  (for _index (range 1 _output_get)
    (set `local.F` true)
    (for _index_2 (range (- (`local.N`) _index)) :!label _label
      (bind _output (`|GetArrayItem` (`local.ListOfTriggeredEnemies`) _index_2))
      (`/Engine/EditorBlueprintResources/StandardMacros.CompareFloat` (`KismetMathLibrary.VSizeXYSquared` (- (`self.K2_GetActorLocation` _output) (`self.K2_GetActorLocation` (`self.As BP Main Character`)))) (`KismetMathLibrary.VSizeXYSquared` (- (`self.K2_GetActorLocation` (`|GetArrayItem` (`local.ListOfTriggeredEnemies`) (+ _index_2 1))) (`self.K2_GetActorLocation` (`self.As BP Main Character`))))
        (:`>`
          (bind _output_get_2 (set `local.SwapEnemy` _output))
          (bind _returnvalue (+ _index_2 1))
          (`KismetArrayLibrary.Array_Set` _listofactiveenemies _index_2 (`|GetArrayItem` _listofactiveenemies _returnvalue))
          (`KismetArrayLibrary.Array_Set` _listofactiveenemies _returnvalue _output_get_2)
          (set `local.F` false))))
    (if (`local.F`)
      (goto _label :!via `Break`))))

(fn `UserConstructionScript`)