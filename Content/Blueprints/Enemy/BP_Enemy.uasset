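; Melee enemy that patrols random points, chases the player when perceived, attacks or backs off, and dies when hitpoints run out.
; Looping timers drive patrol, while perception alerts the EnemyManager and starts a chase.
; MakeDecision picks attack, retreat, chase or patrol from manager-granted permission, range and sight.
; It spawns a hand-socketed weapon with a toggleable hitbox, and plays voices and level-specific footsteps with manual distance-based volume.
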(event `ShouldWalk`
  ;[1 1 1] Если АИ потерял игрока, то этот ивент отправит его патрулировать дальше
  (if (not (`KismetSystemLibrary.K2_IsTimerActiveHandle` (stale `StartWalking` _returnvalue)))
    (bind _doessee (`self.DoesSeePlayer`))
    (if (not _doessee)
      (`KismetSystemLibrary.RetriggerableDelay` 3.0)
      (bind _doessee_2 (`self.DoesSeePlayer`))
      (if (not _doessee_2)
        (`self.StartWalking`)))))

(event `MoveToRandomLocation`
  (bind _currentsoundref (`self.CurrentSoundRef`))
  ;[1 1 1] Включаем AIPerception и идем в патруль
  (set `self.CanDetectPlayer` true)
  (set `CharacterMovementComponent.MaxWalkSpeed` 200.0 (`self.CharacterMovement`))
  (bind _doessee (`self.DoesSeePlayer`))
  (if (not _doessee)
    (`AIBlueprintHelperLibrary.SimpleMoveToLocation` (`AIBlueprintHelperLibrary.GetAIController` self) (`NavigationSystemV1.K2_GetRandomReachablePointInRadius` (`self.K2_GetActorLocation`) 1000.0 null null))
    (`/Engine/EditorBlueprintResources/StandardMacros.IsValid` _currentsoundref
      (:`Is Valid`
        (if (not (`AudioComponent.IsPlaying` _currentsoundref))
          (bind _returnvalue (`GameplayStatics.SpawnSoundAttached` "/Game/FMOD/Assets/New_Folder/Enemies/EnemyVoices.EnemyVoices" (`self.Mesh`) "None" (0.0 0.0 0.0) (struct) "KeepRelativeOffset" false 1.0 1.0 0.0 null null :!label _label))
          (set `self.CurrentSoundRef` _returnvalue)))
      (:`Is Not Valid`
        (goto _label)))))

(event `StartWalking`
  (bind _returnvalue (`KismetSystemLibrary.K2_SetTimerDelegate` (delegate `MoveToRandomLocation`) 2.0 true :!label _label_2)) ; Таймер для патрулирования. Отправляет в рандомную точку каждые 2 секунды
)

(event `self.ReceiveBeginPlay`
  (bind _returnvalue (`self.GetTransform`))
  (`FMODBlueprintStatics.LoadBank` "/Game/FMOD/Banks/Master.Master")
  (bind _returnvalue_2 (`FMODBlueprintStatics.FindEventByName` "SwordSwing"))
  (`FMODBlueprintStatics.PlayEvent2D` _returnvalue_2)
  (`|ExecutionSequence`
    (:`then_0`
      (`KismetSystemLibrary.K2_SetTimerDelegate` (delegate `ShouldWalk`) 4.0 true) ; Таймер для проверки, не стоит ли АИ как дурак без дела
      (goto _label_2))
    (:`then_1`
      ;[1 1 1] Спавним оружие и кидаем его в руку
      (bind _returnvalue_3 (`|SpawnActorFromClass` "/Game/Blueprints/BP_MeleeWeapon.BP_MeleeWeapon_C" (`KismetMathLibrary.MakeTransform` (`KismetMathLibrary.MakeVector` (.x (.location _returnvalue)) (.y (.location _returnvalue)) (- (.z (.location _returnvalue)) 200.0))) "AlwaysSpawn" "OverrideRootScale" null 0 null))
      (set `self.Melee Weapon Ref` _returnvalue_3)
      (`self.K2_AttachToComponent` _returnvalue_3 (`self.Mesh`) "RightHandWeaponSocket" "SnapToTarget" "SnapToTarget" "SnapToTarget" true)
      (`PrimitiveComponent.SetCollisionEnabled` (`/Game/Blueprints/BP_MeleeWeapon.Sphere` _returnvalue_3) "NoCollision")
      (`PrimitiveComponent.SetCollisionEnabled` (`/Game/Blueprints/BP_MeleeWeapon.HitBoxCollision` _returnvalue_3) "NoCollision"))
    (:`then_2`
      (`KismetSystemLibrary.Delay` 1.0)
      (bind _asbp_main_character (cast `/Game/Blueprints/BP_MainCharacter` (`GameplayStatics.GetPlayerCharacter` 0)))
      (bind _output_get (set `self.As BP Main Character` _asbp_main_character))
      (set `self.EnemyManagerRef` (`/Game/Blueprints/BP_MainCharacter.EnemyManagerRef` _output_get)))
    (:`then_3`
      (bind _asbp_game_instance (cast `/Game/Blueprints/Misc/BP_GameInstance` (`GameplayStatics.GetGameInstance`)))
      (set `/Game/Blueprints/Misc/BP_GameInstance.WalkingEnemyRef` self _asbp_game_instance))))

(event `self.AIPerception.OnTargetPerceptionUpdated`
  (params (Actor :type "Actor Object Reference") (Stimulus :type "AIStimulus Structure"))
  (bind _enemymanagerref (`self.EnemyManagerRef`))
  ;[1 1 1] Если АИ заметит игрока, то сообщит менеджеру
  (bind _asbp_main_character (cast `/Game/Blueprints/BP_MainCharacter` Actor))
  (set `self.As BP Main Character` _asbp_main_character)
  (if (`self.CanDetectPlayer`)
    (`/Engine/EditorBlueprintResources/StandardMacros.IsValid` _enemymanagerref
      (:`Is Valid`
        (`/Game/Blueprints/Enemy/BP_EnemyManager.OnEnemyTriggered` _enemymanagerref self)
        ;[1 1 1] Бежим к игроку
        (`/Engine/EditorBlueprintResources/StandardMacros.DoOnce` false :!label _label_3
          (:`Completed`
            (`KismetSystemLibrary.K2_ClearAndInvalidateTimerHandle` (stale `StartWalking` _returnvalue) :!label _label_4)
            (set `CharacterMovementComponent.MaxWalkSpeed` 600.0 (`self.CharacterMovement`))
            (`AITask_MoveTo.AIMoveTo` (`AIBlueprintHelperLibrary.GetAIController` self) (0.0 0.0 0.0) (`self.As BP Main Character`) 100.0 "Disable"
              (:`then`
                (bind _returnvalue (`GameplayStatics.SpawnSoundAttached` "/Game/FMOD/Assets/New_Folder/Footsteps/step_stone_L.step_stone_L" (`self.Mesh`) "None" (0.0 0.0 0.0) (struct) "KeepRelativeOffset" false 0.1 1.0 0.0 null null))
                (set `self.CurrentSoundRef` _returnvalue)
                (bind _returnvalue_2 (`KismetSystemLibrary.K2_SetTimerDelegate` (delegate `PlayFootsteps`) 0.3 true 0.2))
                (set `self.SoundCF` 2.0))
              (:`OnRequestFailed`
                (set `self.IsRetreating` true)
                (`KismetSystemLibrary.Delay` 1.0)
                (set `self.IsRetreating` false)
                (goto _label_3 :!via `Reset`))
              (:`OnMoveFinished`
                (`|ExecutionSequence`
                  (:`then_0`
                    (goto _label_3 :!via `Reset`))
                  (:`then_1`
                    (`self.MakeDecision`)
                    (`KismetSystemLibrary.K2_ClearAndInvalidateTimerHandle` _returnvalue_2)))))))))))

(event `RunToPlayer`
  ;[1 1 1] Бежим к игроку
  (goto _label_4))

(event `CheckIsAttackOver`
  (if (not (`self.IsAttacking`))
    (`KismetSystemLibrary.K2_ClearAndInvalidateTimerHandle` (stale `AttackPlayer` _returnvalue))
    (`KismetSystemLibrary.Delay` 0.2)
    (`self.MakeDecision`)))

(event `AttackPlayer`
  ;[1 1 1] Атакуем игрока
  (set `self.CanDetectPlayer` false)
  (set `CharacterMovementComponent.MaxWalkSpeed` 50.0 (`self.CharacterMovement`))
  (set `self.IsAttacking` true)
  (bind _aswalking_enemy_anim_bp (cast `/Game/Mannequin/Animations/WalkingEnemyAnimBP` (`SkeletalMeshComponent.GetAnimInstance` (`self.Mesh`))))
  (set `/Game/Mannequin/Animations/WalkingEnemyAnimBP.DoesSimpleAttack` true _aswalking_enemy_anim_bp)
  (bind _returnvalue (`KismetSystemLibrary.K2_SetTimerDelegate` (delegate `CheckIsAttackOver`) 0.2 true)))

(event `PlayFootsteps`
  (bind _currentsoundref (`self.CurrentSoundRef`))
  (bind _currentsoundref_2 (`self.CurrentSoundRef`))
  (bind _currentsoundref_3 (`self.CurrentSoundRef`))
  (`/Engine/EditorBlueprintResources/StandardMacros.IsValid` _currentsoundref
    (:`Is Valid`
      (`AudioComponent.Play` _currentsoundref 0.0)
      (bind _returnvalue (`GameplayStatics.GetCurrentLevelName` true))
      (if (`KismetStringLibrary.EqualEqual_StrStr` _returnvalue "TestLevel")
        (switch `int` (`KismetMathLibrary.RandomIntegerInRange` 0 3)
          (:`Default`
            (`AudioComponent.SetSound` _currentsoundref_2 "/Game/FMOD/Assets/New_Folder/Footsteps/step_frozen_L1.step_frozen_L1" :!label _label_5))
          (:`0`
            (goto _label_5))
          (:`1`
            (`AudioComponent.SetSound` _currentsoundref_2 "/Game/FMOD/Assets/New_Folder/Footsteps/step_frozen_L2.step_frozen_L2"))
          (:`2`
            (`AudioComponent.SetSound` _currentsoundref_2 "/Game/FMOD/Assets/New_Folder/Footsteps/step_frozen_R1.step_frozen_R1"))
          (:`3`
            (`AudioComponent.SetSound` _currentsoundref_2 "/Game/FMOD/Assets/New_Folder/Footsteps/Step_frozen_R2.Step_frozen_R2")))
        (else
          (switch `int` (`KismetMathLibrary.RandomIntegerInRange` 0 2)
            (:`Default`
              (`AudioComponent.SetSound` _currentsoundref_3 "/Game/FMOD/Assets/New_Folder/Footsteps/step_stone_R.step_stone_R" :!label _label_6))
            (:`0`
              (goto _label_6))
            (:`1`
              (`AudioComponent.SetSound` _currentsoundref_3 "/Game/FMOD/Assets/New_Folder/Footsteps/step_stone_L2.step_stone_L2"))
            (:`2`
              (`AudioComponent.SetSound` _currentsoundref_3 "/Game/FMOD/Assets/New_Folder/Footsteps/step_stone_R2.step_stone_R2"))))))))

(event `Death`
  ;[1 1 1] Смерть
  (for _array_element (`self.GetAttachedActors` true)
    (`self.K2_DestroyActor` _array_element))
  (`self.K2_DestroyActor`))

(event `Retreat`
  ;[1 1 1] Отступаем
  (set `self.IsRetreating` true)
  (set `self.CanDetectPlayer` false)
  (set `CharacterMovementComponent.MaxWalkSpeed` 100.0 (`self.CharacterMovement`))
  (`AITask_MoveTo.AIMoveTo` (`AIBlueprintHelperLibrary.GetAIController` self) (+ (* (- (`self.K2_GetActorLocation`) (`self.K2_GetActorLocation` (`self.As BP Main Character`))) 2) (`self.K2_GetActorLocation`)) null
    (:`then`
      (bind _returnvalue (`GameplayStatics.SpawnSoundAttached` "/Game/FMOD/Assets/New_Folder/Footsteps/step_stone_L.step_stone_L" (`self.Mesh`) "None" (0.0 0.0 0.0) (struct) "KeepRelativeOffset" false 0.4 1.0 0.0 null null))
      (set `self.CurrentSoundRef` _returnvalue)
      (bind _returnvalue_2 (`KismetSystemLibrary.K2_SetTimerDelegate` (delegate `PlayFootsteps`) 0.3 true 0.2))
      (set `self.SoundCF` 1.0))
    (:`OnRequestFailed`
      (set `self.CanDetectPlayer` true :!label _label_7)
      (set `self.IsRetreating` false)
      (`KismetSystemLibrary.K2_ClearAndInvalidateTimerHandle` _returnvalue_2))
    (:`OnMoveFinished`
      (goto _label_7))))

(event `MakeDecision`
  ;[1 1 1] Проверка что делать атаковать, отступать, бежать к игроку, патрулировать
  (`/Game/Blueprints/Enemy/BP_EnemyManager.GiveOrders` (`self.EnemyManagerRef`))
  (bind _shouldattack (`self.ShouldAttackPlayer?`))
  (if _shouldattack
    (`self.AttackPlayer`)
    (else
      (bind _doessee (`self.DoesSeePlayer`))
      (if _doessee
        (bind _shouldretreat (`self.ShouldRetreat`))
        (if _shouldretreat
          (`self.Retreat`)
          (else
            (`self.RunToPlayer`)))
        (else
          (`self.StartWalking`))))))

(event `self.ReceiveTick`
  (params (DeltaSeconds :type "Float (single-precision)"))
  (bind _as_bp_main_character (`self.As BP Main Character`))
  (bind _currentsoundref (`self.CurrentSoundRef`))
  (bind (_returnvalue_roll _returnvalue_pitch _returnvalue_yaw) (`KismetMathLibrary.BreakRotator` (`KismetMathLibrary.FindLookAtRotation` (`self.K2_GetActorLocation`) (`self.K2_GetActorLocation` _as_bp_main_character))))
  (bind _returnvalue (/ (* (`self.SoundCF`) 15000.0) (`KismetMathLibrary.VSizeSquared` (- (`self.K2_GetActorLocation` (`self.As BP Main Character`)) (`self.K2_GetActorLocation`)))))
  (`|ExecutionSequence`
    (:`then_0`
      ;[1 1 1] Пока враг отступает, он смотрит на ГГ
      (if (`self.IsRetreating`)
        (`/Engine/EditorBlueprintResources/StandardMacros.IsValid` _as_bp_main_character
          (:`Is Valid`
            (`self.K2_SetActorRotation` (`KismetMathLibrary.MakeRotator` 0.0 0.0 _returnvalue_yaw))))))
    (:`then_1`
      ;[1 1 1] Изменяем громкость в зависимости от расстояния до персонажа
      (`/Engine/EditorBlueprintResources/StandardMacros.IsValid` _currentsoundref
        (:`Is Valid`
          (`/Engine/EditorBlueprintResources/StandardMacros.CompareFloat` _returnvalue 1.0
            (:`>`
              (`AudioComponent.SetVolumeMultiplier` _currentsoundref 1.0))
            (:`==`
              (`AudioComponent.SetVolumeMultiplier` _currentsoundref _returnvalue :!label _label_8))
            (:`<`
              (goto _label_8))))))))

(event `StartOfAttack`
  (bind _melee_weapon_ref (`self.Melee Weapon Ref`))
  (`/Engine/EditorBlueprintResources/StandardMacros.IsValid` _melee_weapon_ref
    (:`Is Valid`
      (`PrimitiveComponent.SetCollisionEnabled` (`/Game/Blueprints/BP_MeleeWeapon.HitBoxCollision` _melee_weapon_ref) "QueryOnly"))
    (:`Is Not Valid`
      (`self.FailReport` "NotValid"))))

(event `EndOfAttack`
  (bind _melee_weapon_ref (`self.Melee Weapon Ref`))
  (`/Engine/EditorBlueprintResources/StandardMacros.IsValid` _melee_weapon_ref
    (:`Is Valid`
      (`PrimitiveComponent.SetCollisionEnabled` (`/Game/Blueprints/BP_MeleeWeapon.HitBoxCollision` _melee_weapon_ref) "NoCollision"))))

(event `/Game/Blueprints/BP_WeaponInterface.GetDamage`
  (params (AmountOfDamage :type "Float (single-precision)"))
  ;[1 1 1] Получаем урон через интерфейс
  (bind _output_get (set `self.Hitpoints` (- (`self.Hitpoints`) AmountOfDamage)))
  (`GameplayStatics.PlaySound2D` "/Game/FMOD/Assets/New_Folder/Hits/Flash/wrack.wrack" 1.0 1.0 0.0 null null)
  (if (not (`self.IsAttacking`))
    (bind _aswalking_enemy_anim_bp (cast `/Game/Mannequin/Animations/WalkingEnemyAnimBP` (`SkeletalMeshComponent.GetAnimInstance` (`self.Mesh`))))
    (set `/Game/Mannequin/Animations/WalkingEnemyAnimBP.GotHit` true _aswalking_enemy_anim_bp))
  (`/Engine/EditorBlueprintResources/StandardMacros.CompareFloat` _output_get
    (:`==`
      _)
    (:`<`
      _))
  (`self.Death`))

(fn `DoesSeePlayer`
  (returns (DoesSee :type Boolean))
  (bind _as_bp_main_character (`self.As BP Main Character`))
  (`/Engine/EditorBlueprintResources/StandardMacros.IsValid` _as_bp_main_character
    (:`Is Valid`
      (`/Engine/EditorBlueprintResources/StandardMacros.CompareInt` (`KismetArrayLibrary.Array_Find` (`AIPerceptionComponent.GetCurrentlyPerceivedActors` (`self.AIPerception`) null) _as_bp_main_character)
        (:`>`
          (return true))
        (:`==`
          (return true))
        (:`<`
          _)))
    (:`Is Not Valid`
      _))
  (return false))

(fn `ShouldAttackPlayer?`
  (returns (ShouldAttack :type Boolean))
  (bind _returnvalue (`self.K2_GetActorLocation`))
  (bind _melee_weapon_ref (`self.Melee Weapon Ref`))
  (if (`self.HasPermissionToAttack`)
    (`KismetSystemLibrary.DrawDebugSphere` _returnvalue 150.0 12 (struct :`R` 0.174959 :`G` 1.0 :`A` 1.0) 0.1 1.0)
    (`/Engine/EditorBlueprintResources/StandardMacros.IsValid` _melee_weapon_ref
      (:`Is Valid`
        (bind _outactors (`KismetSystemLibrary.SphereOverlapActors` _returnvalue 150.0 (`|MakeArray` "ObjectTypeQuery3" :!type "EObjectTypeQuery Enum") null (`|MakeArray` self _melee_weapon_ref :!type "Actor Object Reference")))
        (`/Engine/EditorBlueprintResources/StandardMacros.CompareInt` (`KismetArrayLibrary.Array_Find` _outactors (`self.As BP Main Character`))
          (:`>`
            _)
          (:`==`
            _)
          (:`<`
            (return false))))
      (:`Is Not Valid`
        (bind _outactors_2 (`KismetSystemLibrary.SphereOverlapActors` _returnvalue 150.0 (`|MakeArray` "ObjectTypeQuery3" :!type "EObjectTypeQuery Enum") null (`|MakeArray` self :!type "Actor Object Reference")))
        (`/Engine/EditorBlueprintResources/StandardMacros.CompareInt` (`KismetArrayLibrary.Array_Find` _outactors_2 (`self.As BP Main Character`))
          (:`>`
            _)
          (:`==`
            _)
          (:`<`
            (return false)))))
    (return true)
    (else
      (return false))))

(fn `ShouldRetreat`
  (returns (ShouldRetreat :type Boolean))
  (bind _as_bp_main_character (`self.As BP Main Character`))
  (`/Engine/EditorBlueprintResources/StandardMacros.IsValid` _as_bp_main_character
    (:`Is Valid`
      (return (>= 62500.0 (`KismetMathLibrary.VSizeXYSquared` (- (`self.K2_GetActorLocation` _as_bp_main_character) (`self.K2_GetActorLocation`))))))
    (:`Is Not Valid`
      (return false))))

(fn `UserConstructionScript`)