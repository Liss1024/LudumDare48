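; Main player character Blueprint that handles hit points and death, with a helper to check whether an attack montage is active.
; TakeDamage subtracts and prints hit points; below one, it ragdolls the body, face, hands and legs and disables capsule collision and movement.
; Death also fades the camera, shows the WBP_YouDied widget and switches to UI-only input with a visible cursor.
; FailMacro prints failure reasons for debugging.
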(fn `IsAttackMontageActive`
  (returns (ReturnValue :type Boolean))
  (return (`KismetSystemLibrary.IsValid` (`AnimInstance.GetCurrentActiveMontage` (`SkeletalMeshComponent.GetAnimInstance` (`self.Mesh`))))))

(fn `TakeDamage`
  (params (Damage :type "Float (double-precision)"))
  (bind _returnvalue (`GameplayStatics.GetPlayerController` 0))
  (bind _mesh (`self.Mesh`))
  (bind _output_get (set `self.HitPoints` (- (`self.HitPoints`) Damage)))
  (`KismetSystemLibrary.PrintString` (`KismetStringLibrary.Conv_DoubleToString` _output_get))
  (if (> 1.0 (`self.HitPoints`))
    (`PrimitiveComponent.SetCollisionEnabled` (`self.CapsuleComponent`) "NoCollision")
    (`PrimitiveComponent.SetSimulatePhysics` _mesh true)
    (`PrimitiveComponent.SetSimulatePhysics` (`self.Face`) true)
    (`PrimitiveComponent.SetSimulatePhysics` (`self.Hands`) true)
    (`PrimitiveComponent.SetSimulatePhysics` (`self.Legs`) true)
    (`PrimitiveComponent.SetCollisionProfileName` _mesh "Ragdoll" true)
    (`PrimitiveComponent.SetCollisionProfileName` (`self.Face`) "Ragdoll" true)
    (`PrimitiveComponent.SetCollisionProfileName` (`self.Hands`) "Ragdoll" true)
    (`PrimitiveComponent.SetCollisionProfileName` (`self.Legs`) "Ragdoll" true)
    (`CharacterMovementComponent.SetMovementMode` (`self.CharacterMovement`) "MOVE_None" 0)
    (`PlayerCameraManager.StartCameraFade` :`self` (`GameplayStatics.GetPlayerCameraManager` 0) :`FromAlpha` 0.2 :`ToAlpha` 0.9 :`Duration` 2.0 :`bShouldFadeAudio` true :`bHoldWhenFinished` true)
    (bind _returnvalue_2 (`|CreateWidget` "/Game/UI/WBP_YouDied.WBP_YouDied_C"))
    (`UserWidget.AddToViewport` _returnvalue_2 0)
    (`WidgetBlueprintLibrary.SetInputMode_UIOnlyEx` _returnvalue null)
    (set `PlayerController.bShowMouseCursor` true _returnvalue)))

(fn `UserConstructionScript`)